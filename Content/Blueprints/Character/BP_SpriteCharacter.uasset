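; Player-controlled 2D sprite miner that walks along the world Y axis and jumps through Enhanced Input.
; Each tick it picks the idle or walk flipbook from velocity, turns the controller to face the Y movement direction and debug-prints HP.
; When HP reaches zero it flags itself dead, which disables input and switches to the death flipbook; OnReset restores HP and the flag.
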(event `self.ReceiveBeginPlay`
  ;[1 1 1] Event BeginPlay
  (set `self.bIsDead` false)
  (set `self.HP` 1)
  (bind _asplayer_controller (cast `PlayerController` (`self.GetController`)))
  (bind _returnvalue (pcsubsystem `EnhancedInputLocalPlayerSubsystem` _asplayer_controller))
  (`/Engine/EditorBlueprintResources/StandardMacros.IsValid` _returnvalue
    (:`Is Valid`
      (`EnhancedInputSubsystemInterface.AddMappingContext` _returnvalue "/Game/Blueprints/IMC_Movement.IMC_Movement" 0 (struct)))))

(event `self.ReceiveActorBeginOverlap`
  (params (OtherActor :type "Actor Object Reference"))
  ;[1 1 1] Actor Begin Overlap
)

(event `self.ReceiveTick`
  (params (DeltaSeconds :type "Float (single-precision)"))
  ;[1 1 1] Event Tick
  (if (`self.bIsDead`)
    (`self.DisableInput` (`GameplayStatics.GetPlayerController` 0))
    (`PaperFlipbookComponent.SetFlipbook` (`self.Sprite`) "/Game/Sprites/Character/MinerFinal_Death.MinerFinal_Death")
    (else
      (`self.UpdateAnimation`)
      (`self.UpdateRotation`)
      (`KismetSystemLibrary.PrintString` (`KismetStringLibrary.Conv_IntToString` (`self.HP`)) true true (struct :`G` 0.66 :`B` 1.0 :`A` 1.0) 10.0 "1")
      (if (<= (`self.HP`) 0)
        (set `self.bIsDead` true)))))

(event `EnhancedInput|/Game/Blueprints/InputActions/IA_Walk`
  (params (ActionValue :type "Float (double-precision)") (ElapsedSeconds :type "Float (double-precision)") (TriggeredSeconds :type "Float (double-precision)") (InputAction :type "InputAction Object Reference" :default "/Game/Blueprints/InputActions/IA_Walk.IA_Walk"))
  ;[1 1 1] Input Action WALK
  (:`Triggered`
    (`self.AddMovementInput` (0.0 1.0 0.0) ActionValue)))

(event `EnhancedInput|/Game/Blueprints/InputActions/IA_Jump`
  (params (ActionValue :type Boolean) (ElapsedSeconds :type "Float (double-precision)") (TriggeredSeconds :type "Float (double-precision)") (InputAction :type "InputAction Object Reference" :default "/Game/Blueprints/InputActions/IA_Jump.IA_Jump"))
  ;[1 1 1] Input Action JUMP
  (:`Triggered`
    (`self.Jump`))
  (:`Completed`
    (`self.StopJumping`)))

(event `UpdateRotation`
  (bind (_returnvalue_x _returnvalue_y) (`KismetMathLibrary.BreakVector` (`CharacterMovementComponent.GetLastUpdateVelocity` (`self.CharacterMovement`))))
  ;[1 1 1] Update Rotation
  (`/Engine/EditorBlueprintResources/StandardMacros.IsValid` (`self.GetController`)
    (:`Is Valid`
      (`/Engine/EditorBlueprintResources/StandardMacros.CompareFloat` _returnvalue_y
        (:`>`
          (`Controller.SetControlRotation` (`self.GetController`) (`KismetMathLibrary.MakeRotator` 0.0 0.0 90.0)))
        (:`<`
          (`Controller.SetControlRotation` (`self.GetController`) (`KismetMathLibrary.MakeRotator` 0.0 0.0 -90.0)))))))

(event `self.K2_OnReset`
  ;[1 1 1] Event On Reset
  (set `self.bIsDead` false)
  (set `self.HP` 1))

(event `UpdateAnimation`
  ;[1 1 1] Update Animation
  (`PaperFlipbookComponent.SetFlipbook` (`self.Sprite`) (select `bool` (> (`KismetMathLibrary.VSize` (`MovementComponent.Velocity` (`self.CharacterMovement`))) 0.0) :`false` "/Game/Sprites/Character/MinerFinal_Idle.MinerFinal_Idle" :`true` "/Game/Sprites/Character/MinerFinal_Walk.MinerFinal_Walk" :!type "PaperFlipbook Object Reference")))

(fn `UserConstructionScript`)