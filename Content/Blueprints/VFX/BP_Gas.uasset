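; BP_Gas is a VFX actor for a gas effect that starts after a short delay and then drifts through the world.
; BeginPlay adds a Niagara component and holds it inactive.
; Tick accumulates elapsed time in PauseTime through AccumulateTime and, once it passes two seconds, activates the effect and moves the actor along world Y.
; The movement is a fixed offset per frame, not scaled by DeltaSeconds.
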(event `self.ReceiveBeginPlay`
  (set `self.bIsActive` false)
  (set `self.LocationSpeed` 1.0)
  (bind _returnvalue (`AddComponent|NODE_AddNiagaraComponent-0`))
  (`ActorComponent.SetActive` _returnvalue (`self.bIsActive`) false))

(event `self.ReceiveTick`
  (params (DeltaSeconds :type "Float (single-precision)"))
  (if (> (`self.pauseTime`) 2.0)
    (set `self.bIsActive` true)
    (if (`self.bIsActive`)
      (`ActorComponent.SetActive` (stale `self.ReceiveBeginPlay` _returnvalue) (`self.bIsActive`) false)
      (`self.K2_AddActorWorldOffset` (`KismetMathLibrary.MakeVector` 0.0 (`self.LocationSpeed`)))
      (`self.AccumulateTime` DeltaSeconds))
    (else
      (set `self.bIsActive` false)
      (`self.AccumulateTime` DeltaSeconds))))

(fn `AccumulateTime`
  (params (A :type "Float (double-precision)"))
  (set `self.pauseTime` (+ A (`self.pauseTime`))))

(fn `UserConstructionScript`)