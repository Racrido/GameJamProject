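; BP_Collision8 is a lethal collider for the BP_Gas8 gas hazard that sets a BP_SpriteCharacter's HP to zero on overlap.
; Its Cube starts hidden with collision disabled.
; Each Tick looks up BP_Gas8 and, while it is active, shows the Cube, enables overlaps and stretches it along Y at a frame-rate-scaled speed up to a cap, clamping X and Z to fixed values.
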(event `self.ReceiveBeginPlay`
  (set `self.ScaleFactor` 1.5)
  (set `self.PauseTime` 0.0)
  (`SceneComponent.SetVisibility` (`self.Cube`) false false)
  (`PrimitiveComponent.SetCollisionProfileName` (`self.Cube`) "NoCollision" true))

(event `self.ReceiveTick`
  (params (DeltaSeconds :type "Float (single-precision)"))
  (bind _returnvalue (`GameplayStatics.GetActorOfClass` "/Game/Blueprints/VFX/BP_Gas8.BP_Gas8_C"))
  (if (`/Game/Blueprints/VFX/BP_Gas8.bIsActive` _returnvalue)
    (`SceneComponent.SetVisibility` (`self.Cube`) true false)
    (`PrimitiveComponent.SetCollisionProfileName` (`self.Cube`) "OverlapAll" true)
    (`SceneComponent.SetWorldScale3D` (`self.Cube`) (`KismetMathLibrary.MakeVector` (`KismetMathLibrary.FClamp` (.x (+ (`SceneComponent.RelativeScale3D` (`self.Cube`)) (`KismetMathLibrary.MakeVector` 0.0 (`KismetMathLibrary.FClamp` (+ (* (`self.ScaleFactor`) DeltaSeconds) (* 5.0 DeltaSeconds)) 0.0 30.0)))) 1.0) (`KismetMathLibrary.FClamp` (.y (+ (`SceneComponent.RelativeScale3D` (`self.Cube`)) (`KismetMathLibrary.MakeVector` 0.0 (`KismetMathLibrary.FClamp` (+ (* (`self.ScaleFactor`) DeltaSeconds) (* 5.0 DeltaSeconds)) 0.0 30.0)))) 1.0 75.0) (`KismetMathLibrary.FClamp` (.z (+ (`SceneComponent.RelativeScale3D` (`self.Cube`)) (`KismetMathLibrary.MakeVector` 0.0 (`KismetMathLibrary.FClamp` (+ (* (`self.ScaleFactor`) DeltaSeconds) (* 5.0 DeltaSeconds)) 0.0 30.0)))) 2.75 2.75)))))

(event `self.ReceiveActorBeginOverlap`
  (params (OtherActor :type "Actor Object Reference"))
  (bind _asbp_sprite_character (cast `/Game/Blueprints/Character/BP_SpriteCharacter` OtherActor))
  (set `/Game/Blueprints/Character/BP_SpriteCharacter.HP` 0 _asbp_sprite_character))

(fn `UserConstructionScript`)