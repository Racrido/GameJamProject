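; BP_Collision is a growing kill volume, likely the collision for a gas hazard, that sets an overlapping BP_SpriteCharacter's HP to zero.
; After a short pause from BeginPlay, Tick stretches its Cube along Y at a steady, delta-time-scaled rate up to a cap.
; Clamps pin the X and Z scale, so the volume expands on one axis only.
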(event `self.ReceiveBeginPlay`
  (set `self.ScaleFactor` 5.0)
  (set `self.PauseTime` 0.0))

(event `self.ReceiveTick`
  (params (DeltaSeconds :type "Float (single-precision)"))
  (bind _output_get (set `self.PauseTime` (+ (`self.PauseTime`) DeltaSeconds)))
  (if (> _output_get 2.0)
    (`SceneComponent.SetWorldScale3D` (`self.Cube`) (`KismetMathLibrary.MakeVector` (`KismetMathLibrary.FClamp` (.x (+ (`SceneComponent.RelativeScale3D` (`self.Cube`)) (`KismetMathLibrary.MakeVector` 0.0 (`KismetMathLibrary.FClamp` (+ (* (`self.ScaleFactor`) DeltaSeconds) (* 5.0 DeltaSeconds)) 0.0 30.0)))) 1.0) (`KismetMathLibrary.FClamp` (.y (+ (`SceneComponent.RelativeScale3D` (`self.Cube`)) (`KismetMathLibrary.MakeVector` 0.0 (`KismetMathLibrary.FClamp` (+ (* (`self.ScaleFactor`) DeltaSeconds) (* 5.0 DeltaSeconds)) 0.0 30.0)))) 1.0 75.0) (`KismetMathLibrary.FClamp` (.z (+ (`SceneComponent.RelativeScale3D` (`self.Cube`)) (`KismetMathLibrary.MakeVector` 0.0 (`KismetMathLibrary.FClamp` (+ (* (`self.ScaleFactor`) DeltaSeconds) (* 5.0 DeltaSeconds)) 0.0 30.0)))) 2.75 2.75)))))

(event `self.ReceiveHit`
  (params (MyComp :type "PrimitiveComponent Object Reference") (Other :type "Actor Object Reference") (OtherComp :type "PrimitiveComponent Object Reference") (bSelfMoved :type Boolean) (HitLocation :type "Vector Structure") (HitNormal :type "Vector Structure") (NormalImpulse :type "Vector Structure") (Hit :type "HitResult Structure (by ref)")))

(event `self.ReceiveActorBeginOverlap`
  (params (OtherActor :type "Actor Object Reference"))
  (bind _asbp_sprite_character (cast `/Game/Blueprints/Character/BP_SpriteCharacter` OtherActor))
  (set `/Game/Blueprints/Character/BP_SpriteCharacter.HP` 0 _asbp_sprite_character))

(fn `UserConstructionScript`)